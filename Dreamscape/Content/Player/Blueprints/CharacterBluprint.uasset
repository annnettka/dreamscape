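; Player character Blueprint that handles basic walk and mouse-look controls through input axis events.
; Forward/back and left/right axes store their values and add movement input along the control rotation's forward and right vectors.
; The forward direction uses the full control rotation rather than yaw alone, so it includes camera pitch.
; Mouse X and Y axes feed controller yaw and pitch directly, without sensitivity scaling.
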(event Input|AxisEvents|InputAxisForwardBackInput
  (params (AxisValue :type Float%20%28single-precision%29))
  (bind _output_get (Variables|Default|SetForwardBackScale AxisValue))
  (Pawn|Input|AddMovementInput (Math|Vector|GetForwardVector (Pawn|GetControlRotation :!class /Script/Engine.Pawn)) _output_get false))

(event Input|AxisEvents|InputAxisLeftRightInput
  (params (AxisValue :type Float%20%28single-precision%29))
  (bind _output_get (Variables|Default|SetLeftRightScale AxisValue))
  (Pawn|Input|AddMovementInput (Math|Vector|GetRightVector (Pawn|GetControlRotation :!class /Script/Engine.Pawn)) _output_get false))

(event Input|AxisEvents|InputAxisMouseMovementX
  (params (AxisValue :type Float%20%28single-precision%29))
  (Pawn|Input|AddControllerYawInput AxisValue))

(event Input|AxisEvents|InputAxisMouseMovementY
  (params (AxisValue :type Float%20%28single-precision%29))
  (Pawn|Input|AddControllerPitchInput AxisValue))

(fn ConstructionScript)